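; Node actor, apparently for a VR node visualization, that carries a Mass value and displays it on a text render set in the construction script.
; GenCOM computes the mass-weighted average position of an array of basicNode actors.
; BeginPlay, overlap and Tick are empty.
; Disconnected logic would swap 2D and 3D parts by distance to the MotionControllerPawn and turn distant nodes toward it after a distance-scaled delay.
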(event `self.ReceiveBeginPlay`)

(event `self.ReceiveActorBeginOverlap`
  (params (OtherActor :type "Actor Object Reference")))

(event `self.ReceiveTick`
  (params (DeltaSeconds :type "Float (single-precision)")))

(fn `Gen COM`
  (params (NewParam :type "Array of Actor Object Reference"))
  (returns (NewParam1 :type "Vector Structure"))
  (locals (xPos :type "Float (double-precision)") (yPos :type "Float (double-precision)") (zPos :type "Float (double-precision)") (denominator :type "Float (double-precision)") (newCOM :type "Vector Structure"))
  (bind _denominator (`local.denominator`))
  (for _array_element NewParam
    (bind _asbasic_node (cast `/Game/nodes/blueprints/nodeClasses/basicNode` _array_element)
      (:`then`
        (bind _mass (`/Game/nodes/blueprints/nodeClasses/basicNode.mass` _asbasic_node))
        (set `local.xPos` (+ (* _mass (.x (`self.K2_GetActorLocation` _asbasic_node))) (`local.xPos`)))
        (set `local.yPos` (+ (* _mass (.y (`self.K2_GetActorLocation` _asbasic_node))) (`local.yPos`)))
        (set `local.zPos` (+ (* _mass (.z (`self.K2_GetActorLocation` _asbasic_node))) (`local.zPos`)))
        (set `local.denominator` (+ (`local.denominator`) _mass)))
      (:`CastFailed`
        (`KismetSystemLibrary.PrintString` "fucking shit"))))
  (bind _output_get (set `local.newCOM` (`KismetMathLibrary.MakeVector` (/ (`local.xPos`) _denominator) (/ (`local.yPos`) _denominator) (/ (`local.zPos`) _denominator))))
  (return _output_get))

(fn `UserConstructionScript`
  (`TextRenderComponent.K2_SetText` (`self.TextRender`) (`KismetTextLibrary.Conv_DoubleToText` (`self.mass`) "HalfToEven")))