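; A VR node actor that shows its Mass as text and swaps between 2D and 3D parts by distance to the player's MotionControllerPawn.
; When far, Tick turns it toward the pawn's camera or VR target, throttled by a movement threshold and delay that both grow with distance as a cheap billboard LOD.
; GenCOM separately computes a mass-weighted center from supplied basicNode actors.
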(event `self.ReceiveBeginPlay`)

(event `self.ReceiveActorBeginOverlap`
  (params (OtherActor :type "Actor Object Reference")))

(event `self.ReceiveTick`
  (params (DeltaSeconds :type "Float (single-precision)"))
  (bind _returnvalue (`self.K2_GetActorLocation`))
  (bind _returnvalue_2 (`self.K2_GetActorLocation` self))
  (bind _asmotion_controller_pawn (cast `/Game/VirtualRealityBP/Blueprints/MotionControllerPawn` (`GameplayStatics.GetPlayerPawn` 0)))
  (bind _returnvalue_3 (`SceneComponent.K2_GetComponentLocation` (`/Game/VirtualRealityBP/Blueprints/MotionControllerPawn.vrTarget` _asmotion_controller_pawn)))
  (bind _returnvalue_4 (`KismetMathLibrary.Vector_Distance` _returnvalue_3 _returnvalue))
  (if (> _returnvalue_4 1000.0)
    (if (`self.3d`)
      (`SceneComponent.SetVisibility` (`self.2dPart`) true false)
      (`SceneComponent.SetVisibility` (`self.3dPart`) false false)
      (set `self.3d` false))
    (if (not (== (`self.previousLocation`) _returnvalue_3 :`ErrorTolerance` (/ _returnvalue_4 2.0)))
      (set `self.previousLocation` _returnvalue_3)
      (bind _output_get (set `self.delayAmount` (* _returnvalue_4 0.002)))
      (`KismetSystemLibrary.Delay` (+ _output_get (/ (`self.delayAmount`) 5.0)))
      (if (< _returnvalue_4 1500.0)
        (`self.K2_SetActorRotation` (`KismetMathLibrary.Conv_VectorToRotator` (`KismetMathLibrary.GreaterGreater_VectorRotator` (`KismetMathLibrary.Normal` (* (- (`SceneComponent.K2_GetComponentLocation` (`/Game/VirtualRealityBP/Blueprints/MotionControllerPawn.cameraTarget` _asmotion_controller_pawn)) (`self.K2_GetActorLocation`)) (1.0 1.0 1.0))))))
        (else
          (`self.K2_SetActorRotation` (`KismetMathLibrary.Conv_VectorToRotator` (`KismetMathLibrary.GreaterGreater_VectorRotator` (`KismetMathLibrary.Normal` (* (- _returnvalue_3 _returnvalue) (1.0 1.0 1.0))))))))
      (if false
        (`KismetSystemLibrary.LineTraceSingle` :`Start` _returnvalue_2 :`End` (+ _returnvalue_2 (* (`self.GetActorForwardVector` self) 10000.0)) :`TraceChannel` "TraceTypeQuery2" :`DrawDebugType` "ForDuration" :`TraceColor` (struct :`G` 1.0 :`B` 1.0 :`A` 1.0) :`TraceHitColor` (struct :`G` 1.0 :`B` 1.0 :`A` 1.0) :`DrawTime` (/ (`self.delayAmount`) 1.5))))
    (else
      (`SceneComponent.SetVisibility` (`self.3dPart`) true false)
      (`SceneComponent.SetVisibility` (`self.2dPart`) false false)
      (set `self.3d` true))))

(fn `Gen COM`
  (params (NewParam :type "Array of Actor Object Reference"))
  (returns (NewParam1 :type "Vector Structure"))
  (locals (xPos :type "Float (double-precision)") (yPos :type "Float (double-precision)") (zPos :type "Float (double-precision)") (denominator :type "Float (double-precision)") (newCOM :type "Vector Structure"))
  (bind _denominator (`local.denominator`))
  (for _array_element NewParam
    (bind _asbasic_node (cast `/Game/nodes/blueprints/nodeClasses/basicNode` _array_element)
      (:`then`
        (bind _mass (`/Game/nodes/blueprints/nodeClasses/basicNode.mass` _asbasic_node))
        (set `local.xPos` (+ (* _mass (.x (`self.K2_GetActorLocation` _asbasic_node))) (`local.xPos`)))
        (set `local.yPos` (+ (* _mass (.y (`self.K2_GetActorLocation` _asbasic_node))) (`local.yPos`)))
        (set `local.zPos` (+ (* _mass (.z (`self.K2_GetActorLocation` _asbasic_node))) (`local.zPos`)))
        (set `local.denominator` (+ (`local.denominator`) _mass)))
      (:`CastFailed`
        (`KismetSystemLibrary.PrintString` "fucking shit"))))
  (bind _output_get (set `local.newCOM` (`KismetMathLibrary.MakeVector` (/ (`local.xPos`) _denominator) (/ (`local.yPos`) _denominator) (/ (`local.zPos`) _denominator))))
  (return _output_get))

(fn `UserConstructionScript`
  (`TextRenderComponent.K2_SetText` (`self.TextRender`) (`KismetTextLibrary.Conv_DoubleToText` (`self.mass`) "HalfToEven")))